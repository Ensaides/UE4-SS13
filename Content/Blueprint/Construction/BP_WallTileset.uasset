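; BP_WallTileset is an editor-time construction tile that places WallClass actors on the open sides of a 256-unit square.
; The construction script calls Refresh, which destroys the stored walls, queries GetOverlaps, and uses SpawnActorInEditor to spawn a rotated wall on each side without an overlap.
; DestroyWalls and PrintDebugInfo bools act as self-resetting buttons that clear the walls or print tile info during construction.
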(event EventBeginPlay)

(event Collision|EventActorBeginOverlap
  (params (OtherActor :type Actor%20Object%20Reference)))

(event EventTick
  (params (DeltaSeconds :type Float%20%28single-precision%29)))

(event EventRefresh
  (params (bRefreshAdjacent :type Boolean))
  (bind _returnvalue (Transformation|GetActorTransform))
  (bind _wallclass (Variables|Default|GetWallClass))
  (bind (_location _rotation _scale) (Math|Transform|BreakTransform _returnvalue))
  (CallFunction|DestroyWalls)
  (bind _returnvalue_2 (Class|WallTileset|GetOverlaps bRefreshAdjacent))
  (Utilities|FlowControl|Sequence
    (:then_0
      (if (not (.bUpOverlap (Utilities|Struct|BreakWallTilesetOverlaps _returnvalue_2)))
        (bind _returnvalue_3 (Class|Tileset|SpawnActorinEditor _wallclass (Math|Transform|MakeTransform (+ _location "0,256.000000,0.000000") (Math|Rotator|CombineRotators _rotation "0, 0, 0") _scale)))
        (Variables|Default|SetUp _returnvalue_3)))
    (:then_1
      (if (not (.bDownOverlap (Utilities|Struct|BreakWallTilesetOverlaps _returnvalue_2)))
        (bind _returnvalue_4 (Class|Tileset|SpawnActorinEditor _wallclass (Math|Transform|MakeTransform (+ _location "256.000000,0.000000, 0") (Math|Rotator|CombineRotators _rotation "0.000000,180.000000,0.000000") _scale)))
        (Variables|Default|SetDown _returnvalue_4)))
    (:then_2
      (if (not (.bLeftOverlap (Utilities|Struct|BreakWallTilesetOverlaps _returnvalue_2)))
        (bind _returnvalue_5 (Class|Tileset|SpawnActorinEditor _wallclass (Math|Transform|MakeTransform (+ _location "0.000000,0.000000,0.000000") (Math|Rotator|CombineRotators _rotation "0,90.000000, 0") _scale)))
        (Variables|Default|SetLeft _returnvalue_5)))
    (:then_3
      (if (not (.bRightOverlap (Utilities|Struct|BreakWallTilesetOverlaps _returnvalue_2)))
        (bind _returnvalue_6 (Class|Tileset|SpawnActorinEditor _wallclass (Math|Transform|MakeTransform (+ _location "256.000000,256.000000, 0") (Math|Rotator|CombineRotators _rotation "0,-90.000000, 0") _scale)))
        (Variables|Default|SetRight _returnvalue_6)))))

(fn ConstructionScript
  (Utilities|FlowControl|Sequence
    (:then_0
      (if (Variables|Default|GetbDestroyWalls)
        (CallFunction|DestroyWalls)
        (Variables|Default|SetbDestroyWalls false)
        (else
          (Class|Tileset|Refresh false))))
    (:then_1
      (if (Variables|Default|GetbPrintDebugInfo)
        (Class|TilesetManager|PrintTileInfo)
        (Variables|Default|SetbPrintDebugInfo false)))))

(fn DestroyWalls
  (Utilities|FlowControl|Sequence
    (:then_0
      (Utilities|IsValid (Variables|Default|GetUp)
        (:Is%20Valid
          (Actor|DestroyActor (Variables|Default|GetUp))
          (Variables|Default|SetUp 0))))
    (:then_1
      (Utilities|IsValid (Variables|Default|GetDown)
        (:Is%20Valid
          (Actor|DestroyActor (Variables|Default|GetDown))
          (Variables|Default|SetDown 0))))
    (:then_2
      (Utilities|IsValid (Variables|Default|GetLeft)
        (:Is%20Valid
          (Actor|DestroyActor (Variables|Default|GetLeft))
          (Variables|Default|SetLeft 0))))
    (:then_3
      (Utilities|IsValid (Variables|Default|GetRight)
        (:Is%20Valid
          (Actor|DestroyActor (Variables|Default|GetRight))
          (Variables|Default|SetRight 0))))))