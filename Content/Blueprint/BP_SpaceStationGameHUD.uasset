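; Space station game HUD that hosts the player's chat window.
; SetupChatWindow creates a Chat widget for the owning player, stores it and passes it to SetChatWindowContent, while AddChatMessage forwards new messages to that widget.
; OpenRoundStartMenu is an empty event; the logic that creates and displays the RoundStartMenu widget is disconnected and never runs.
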(event EventBeginPlay)

(event Collision|EventActorBeginOverlap
  (params (OtherActor :type Actor%20Object%20Reference)))

(event EventOpenRoundStartMenu)

(event EventSetupChatWindow
  (bind _returnvalue (UserInterface|CreateWidget "/Game/Blueprint/UI/Blueprints/Chat/Chat.Chat_C" (Game|Player|GetOwningPlayerController)))
  (bind _output_get (Variables|Default|SetChatWindowWidget _returnvalue))
  (Class|SpaceStationGameHUD|SetChatWindowContent _output_get))

(event EventAddChatMessage
  (params (NewMessage :type Client%20Chat%20Message%20Struct%20Structure))
  (Default|AddMessage (Variables|Default|GetChatWindowWidget) NewMessage))

(fn ConstructionScript)